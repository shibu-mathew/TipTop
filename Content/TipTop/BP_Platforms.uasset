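; BP_Platforms is a platform actor that dips briefly in response to the player character touching it.
; It stores its root's relative location at BeginPlay as the resting position.
; When BP_ThirdPersonCharacter overlaps the Box, a short delay precedes the Timeline_Bounce playback, whose curve lerps the root's Z between rest and a slightly lower point.
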(event OnComponentBeginOverlap(Box)
  (params (OverlappedComponent :type Primitive%20Component%20Object%20Reference) (OtherActor :type Actor%20Object%20Reference) (OtherComp :type Primitive%20Component%20Object%20Reference) (OtherBodyIndex :type Integer) (bFromSweep :type Boolean) (SweepResult :type Hit%20Result%20Structure%20%28by%20ref%29))
  (bind _new_location (Variables|Default|GetNew%20Location))
  (Utilities|Casting|CastToBP_ThirdPersonCharacter OtherActor)
  (Utilities|FlowControl|Delay 0.5)
  (bind _bounce (Timeline|Timeline_Bounce PlayFromStart)
    (:Update
      (Transformation|SetRelativeLocation (Variables|Default|GetDefaultSceneRoot) (Math|Vector|MakeVector (.x _new_location) (.y _new_location) (Math|Float|Lerp (.z _new_location) (+ (.z _new_location) -1e+01) _bounce)) false false))))

(event EventBeginPlay
  (Variables|Default|SetNew%20Location (Variables|/Script/Engine.SceneComponent|GetRelativeLocation (Variables|Default|GetDefaultSceneRoot))))

(event Collision|EventActorBeginOverlap
  (params (OtherActor :type Actor%20Object%20Reference)))

(event EventTick
  (params (DeltaSeconds :type Float%20%28single-precision%29)))

(fn ConstructionScript)